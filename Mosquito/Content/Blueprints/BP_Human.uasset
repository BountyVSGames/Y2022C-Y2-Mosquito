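; BP_Human is a human actor that dies on any overlap with its capsule, ragdolls and is then removed.
; BeginPlay enables query and physics collision on the skeletal mesh, and the capsule overlap sets IsDead without filtering the other actor.
; Tick polls that flag and, if the mesh already reports gravity enabled, turns on physics simulation and gravity, then destroys the actor after a short delay.
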(event OnComponentBeginOverlap(Capsule)
  (params (OverlappedComponent :type Primitive%20Component%20Object%20Reference) (OtherActor :type Actor%20Object%20Reference) (OtherComp :type Primitive%20Component%20Object%20Reference) (OtherBodyIndex :type Integer) (bFromSweep :type Boolean) (SweepResult :type Hit%20Result%20Structure%20%28by%20ref%29))
  (Variables|Default|SetIsDead true))

(event EventBeginPlay
  (Collision|SetCollisionEnabled (Variables|Default|GetSkeletalMesh) "QueryAndPhysics"))

(event Collision|EventActorBeginOverlap
  (params (OtherActor :type Actor%20Object%20Reference)))

(event EventTick
  (params (DeltaSeconds :type Float%20%28single-precision%29))
  (bind _skeletalmesh (Variables|Default|GetSkeletalMesh))
  (if (and (Variables|Default|GetIsDead) (Class|PrimitiveComponent|IsGravityEnabled _skeletalmesh))
    (Physics|SetSimulatePhysics _skeletalmesh true)
    (Physics|SetEnableGravity _skeletalmesh true)
    (Utilities|FlowControl|Delay 5.0)
    (Actor|DestroyActor)))

(fn ConstructionScript)